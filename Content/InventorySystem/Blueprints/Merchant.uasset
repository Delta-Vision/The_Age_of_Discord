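; Merchant actor that opens a shop for either the global-map or local-map player character.
; A sphere overlap registers it as the character's NearbyMerchant and toggles its text prompt.
; Interact, gated by a DoOnce, creates a centered ShopWidget, refreshes the inventory, flags the shop open and stops movement.
; OnShopClosed restores walking, refreshes any visible inventory, removes the widget and resets the DoOnce.
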(event OnComponentBeginOverlap(Sphere)
  (params (OverlappedComponent :type Primitive%20Component%20Object%20Reference) (OtherActor :type Actor%20Object%20Reference) (OtherComp :type Primitive%20Component%20Object%20Reference) (OtherBodyIndex :type Integer) (bFromSweep :type Boolean) (SweepResult :type Hit%20Result%20Structure%20%28by%20ref%29))
  (Utilities|FlowControl|Sequence
    (:then_0
      (bind _asglobal_map_character (Utilities|Casting|CastToGlobalMapCharacter OtherActor))
      (Variables|/Game/Characters/GlobalMapCharacter/GlobalMapCharacter.GlobalMapCharacter_C|SetNearbyMerchant _asglobal_map_character self)
      (Rendering|SetVisibility (Variables|Default|GetMerchantText) true false))
    (:then_1
      (bind _aslocal_map_character (Utilities|Casting|CastToLocalMapCharacter OtherActor))
      (Variables|/Game/Characters/LocalMapCharacter/LocalMapCharacter.LocalMapCharacter_C|SetNearbyMerchant _aslocal_map_character self)
      (Rendering|SetVisibility (Variables|Default|GetMerchantText) true false))))

(event OnComponentEndOverlap(Sphere)
  (params (OverlappedComponent :type Primitive%20Component%20Object%20Reference) (OtherActor :type Actor%20Object%20Reference) (OtherComp :type Primitive%20Component%20Object%20Reference) (OtherBodyIndex :type Integer))
  (Utilities|FlowControl|Sequence
    (:then_0
      (bind _asglobal_map_character (Utilities|Casting|CastToGlobalMapCharacter OtherActor))
      (Variables|/Game/Characters/GlobalMapCharacter/GlobalMapCharacter.GlobalMapCharacter_C|SetNearbyMerchant _asglobal_map_character 0)
      (Rendering|SetVisibility (Variables|Default|GetMerchantText) false false))
    (:then_1
      (bind _aslocal_map_character (Utilities|Casting|CastToLocalMapCharacter OtherActor))
      (Variables|/Game/Characters/LocalMapCharacter/LocalMapCharacter.LocalMapCharacter_C|SetNearbyMerchant _aslocal_map_character 0)
      (Rendering|SetVisibility (Variables|Default|GetMerchantText) false false))))

(event Custom|Interact
  (params (GlobalMapCharacter :type Global%20Map%20Character%20Object%20Reference) (LocalMapCharacter :type Local%20Map%20Character%20Object%20Reference))
  (Utilities|FlowControl|DoOnce false
    (:Completed
      (Utilities|IsValid GlobalMapCharacter
        (:Is%20Valid
          (Variables|Default|SetGlobalCharacterCharacter GlobalMapCharacter)
          (bind _returnvalue (UserInterface|CreateWidget "/Game/InventorySystem/Widgets/ShopWidget.ShopWidget_C" 0 self (Variables|Default|GetGlobalCharacterCharacter) 0))
          (Variables|Default|SetShopWidget _returnvalue))
        (:Is%20Not%20Valid
          (Variables|Default|SetLocalMapCharacter LocalMapCharacter)
          (bind _returnvalue_2 (UserInterface|CreateWidget "/Game/InventorySystem/Widgets/ShopWidget.ShopWidget_C" 0 self (Variables|Default|GetGlobalCharacterCharacter) (Variables|Default|GetLocalMapCharacter)))
          (Variables|Default|SetShopWidget _returnvalue_2)))
      (Class|UserWidget|SetPositioninViewport :self (Variables|Default|GetShopWidget) :bRemoveDPIScale false)
      (Class|UserWidget|SetAnchorsinViewport (Variables|Default|GetShopWidget) (Utilities|Struct|MakeAnchors "(X=0.500000,Y=0.500000)" "(X=0.500000,Y=0.500000)"))
      (Class|UserWidget|SetAlignmentinViewport (Variables|Default|GetShopWidget) "(X=0.500000,Y=0.500000)")
      (UserInterface|Viewport|AddtoViewport (Variables|Default|GetShopWidget) 5)
      (Utilities|IsValid (Variables|Default|GetGlobalCharacterCharacter)
        (:Is%20Valid
          (Default|HideInventory (Variables|/Game/Characters/GlobalMapCharacter/GlobalMapCharacter.GlobalMapCharacter_C|GetInventoryRef (Variables|Default|GetGlobalCharacterCharacter)))
          (Default|ShowInventory (Variables|/Game/Characters/GlobalMapCharacter/GlobalMapCharacter.GlobalMapCharacter_C|GetInventoryRef (Variables|Default|GetGlobalCharacterCharacter)))
          (Variables|/Game/Characters/GlobalMapCharacter/GlobalMapCharacter.GlobalMapCharacter_C|SetIsShopIsOpen? (Variables|Default|GetGlobalCharacterCharacter) true)
          (Pawn|Components|CharacterMovement|DisableMovement (Variables|/Script/Engine.Character|GetCharacterMovement (Variables|Default|GetGlobalCharacterCharacter)))
          (Components|Movement|StopMovementImmediately (Variables|/Script/Engine.Character|GetCharacterMovement (Variables|Default|GetGlobalCharacterCharacter))))
        (:Is%20Not%20Valid
          (Default|HideInventory (Variables|/Game/Characters/LocalMapCharacter/LocalMapCharacter.LocalMapCharacter_C|GetInventoryRef (Variables|Default|GetLocalMapCharacter)))
          (Default|ShowInventory (Variables|/Game/Characters/LocalMapCharacter/LocalMapCharacter.LocalMapCharacter_C|GetInventoryRef (Variables|Default|GetLocalMapCharacter)))
          (Variables|/Game/Characters/LocalMapCharacter/LocalMapCharacter.LocalMapCharacter_C|SetIsShopIsOpen? (Variables|Default|GetLocalMapCharacter) true)
          (Pawn|Components|CharacterMovement|DisableMovement (Variables|/Script/Engine.Character|GetCharacterMovement (Variables|Default|GetLocalMapCharacter)))
          (Components|Movement|StopMovementImmediately (Variables|/Script/Engine.Character|GetCharacterMovement (Variables|Default|GetLocalMapCharacter))))))))

(event Custom|OnShopClosed
  (Utilities|IsValid (Variables|Default|GetGlobalCharacterCharacter)
    (:Is%20Valid
      (Variables|/Game/Characters/GlobalMapCharacter/GlobalMapCharacter.GlobalMapCharacter_C|SetIsShopIsOpen? (Variables|Default|GetGlobalCharacterCharacter) false)
      (Pawn|Components|CharacterMovement|SetMovementMode (Variables|/Script/Engine.Character|GetCharacterMovement (Variables|Default|GetGlobalCharacterCharacter)) "MOVE_Walking" 0)
      (if (Variables|/Game/InventorySystem/Blueprints/BP_Inventory.BP_Inventory_C|GetIsVisible? (Variables|/Game/Characters/GlobalMapCharacter/GlobalMapCharacter.GlobalMapCharacter_C|GetInventoryRef (Variables|Default|GetGlobalCharacterCharacter)))
        (Default|HideInventory (Variables|/Game/Characters/GlobalMapCharacter/GlobalMapCharacter.GlobalMapCharacter_C|GetInventoryRef (Variables|Default|GetGlobalCharacterCharacter)))
        (Default|ShowInventory (Variables|/Game/Characters/GlobalMapCharacter/GlobalMapCharacter.GlobalMapCharacter_C|GetInventoryRef (Variables|Default|GetGlobalCharacterCharacter))))
      (Widget|RemovefromParent (Variables|Default|GetShopWidget))
      (Variables|Default|SetShopWidget 0)
      (Utilities|FlowControl|DoOnce false) ; enters at Reset
    )
    (:Is%20Not%20Valid
      (Variables|/Game/Characters/LocalMapCharacter/LocalMapCharacter.LocalMapCharacter_C|SetIsShopIsOpen? (Variables|Default|GetLocalMapCharacter) false)
      (Pawn|Components|CharacterMovement|SetMovementMode (Variables|/Script/Engine.Character|GetCharacterMovement (Variables|Default|GetLocalMapCharacter)) "MOVE_Walking" 0)
      (if (Variables|/Game/InventorySystem/Blueprints/BP_Inventory.BP_Inventory_C|GetIsVisible? (Variables|/Game/Characters/LocalMapCharacter/LocalMapCharacter.LocalMapCharacter_C|GetInventoryRef (Variables|Default|GetLocalMapCharacter)))
        (Default|HideInventory (Variables|/Game/Characters/LocalMapCharacter/LocalMapCharacter.LocalMapCharacter_C|GetInventoryRef (Variables|Default|GetLocalMapCharacter)))
        (Default|ShowInventory (Variables|/Game/Characters/LocalMapCharacter/LocalMapCharacter.LocalMapCharacter_C|GetInventoryRef (Variables|Default|GetLocalMapCharacter))))
      (Widget|RemovefromParent (Variables|Default|GetShopWidget))
      (Variables|Default|SetShopWidget 0)
      (Utilities|FlowControl|DoOnce false) ; enters at Reset
    )))

(fn ConstructionScript)