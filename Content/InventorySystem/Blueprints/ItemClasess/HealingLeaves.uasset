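; HealingLeaves is a consumable inventory item that restores a fixed amount of health when used.
; On use, it targets the inventory's global map character if valid, otherwise the local map character.
; If that character is below max HP, it heals them and removes one unit from its inventory slot.
; The item actor destroys itself either way, so at full health nothing is consumed.
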(event EventBeginPlay
  (|CallParentFunction))

(event Collision|EventActorBeginOverlap
  (params (OtherActor :type Actor%20Object%20Reference))
  (|CallParentFunction OtherActor))

(event EventTick
  (params (DeltaSeconds :type Float%20%28single-precision%29))
  (|CallParentFunction DeltaSeconds))

(event EventEventonUsed
  (bind _inventory (Variables|Default|GetInventory))
  (bind _inventory_2 (Variables|Default|GetInventory))
  (bind _localmapcharacter (Variables|/Game/InventorySystem/Blueprints/BP_Inventory.BP_Inventory_C|GetLocalMapCharacter _inventory))
  (bind _globalmapcharacter (Variables|/Game/InventorySystem/Blueprints/BP_Inventory.BP_Inventory_C|GetGlobalMapCharacter _inventory_2))
  (Utilities|IsValid (Variables|/Game/InventorySystem/Blueprints/BP_Inventory.BP_Inventory_C|GetGlobalMapCharacter (Variables|Default|GetInventory))
    (:Is%20Valid
      (if (< (Variables|/Game/Characters/GlobalMapCharacter/GlobalMapCharacter.GlobalMapCharacter_C|GetCurrentHp _globalmapcharacter) (Variables|/Game/Characters/GlobalMapCharacter/GlobalMapCharacter.GlobalMapCharacter_C|GetMaxHP _globalmapcharacter))
        (Default|IncreaseHealth _globalmapcharacter 10)
        (Default|RemoveItematIndex (Variables|Default|GetInventory) (Variables|Default|GetIndex) 1)
        (Actor|DestroyActor)
        (else
          (Actor|DestroyActor))))
    (:Is%20Not%20Valid
      (if (< (Variables|/Game/Characters/LocalMapCharacter/LocalMapCharacter.LocalMapCharacter_C|GetCurrentHp _localmapcharacter) (Variables|/Game/Characters/LocalMapCharacter/LocalMapCharacter.LocalMapCharacter_C|GetMaxHP _localmapcharacter))
        (Default|IncreaseHealth _localmapcharacter 10)
        (Default|RemoveItematIndex (Variables|Default|GetInventory) (Variables|Default|GetIndex) 1)
        (Actor|DestroyActor)
        (else
          (Actor|DestroyActor))))))

(fn ConstructionScript
  (|CallParentFunction))