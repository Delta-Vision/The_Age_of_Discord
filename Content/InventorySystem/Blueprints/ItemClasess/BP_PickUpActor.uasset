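; World pickup actor that adds an item stack to the inventory of a global-map or local-map character.
; Construction takes mesh, scale and interact radius from the item class defaults.
; Sphere overlap triggers a commanded pickup or queues the actor in the character's nearby list, whose first entry shows the name label.
; Pickup records the remaining amount by ID and destroys emptied actors; cursor hover highlights only with a global-map character present.
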(event OnBeginCursorOver(StatickMesh)
  (params (TouchedComponent :type Primitive%20Component%20Object%20Reference))
  (Utilities|IsValid (Variables|Default|GetGlobalMapCharacter)
    (:Is%20Valid
      (CallFunction|OnHovered))))

(event OnComponentEndOverlap(Sphere)
  (params (OverlappedComponent :type Primitive%20Component%20Object%20Reference) (OtherActor :type Actor%20Object%20Reference) (OtherComp :type Primitive%20Component%20Object%20Reference) (OtherBodyIndex :type Integer))
  (Utilities|FlowControl|Sequence
    (:then_0
      (bind _asglobal_map_character (Utilities|Casting|CastToGlobalMapCharacter OtherActor))
      (Variables|Default|SetIsInRange? false)
      (if (and (Utilities|IsValid (Utilities|Array|Get(acopy) (Variables|/Game/Characters/GlobalMapCharacter/GlobalMapCharacter.GlobalMapCharacter_C|GetNearbyPickupActors _asglobal_map_character))) (== (Utilities|Array|Get(acopy) (Variables|/Game/Characters/GlobalMapCharacter/GlobalMapCharacter.GlobalMapCharacter_C|GetNearbyPickupActors _asglobal_map_character)) self))
        (Rendering|SetVisibility (Variables|Default|GetPickUpText) false false)
        (Utilities|Array|RemoveItem (Variables|/Game/Characters/GlobalMapCharacter/GlobalMapCharacter.GlobalMapCharacter_C|GetNearbyPickupActors _asglobal_map_character) self)
        (Utilities|IsValid (Utilities|Array|Get(acopy) (Variables|/Game/Characters/GlobalMapCharacter/GlobalMapCharacter.GlobalMapCharacter_C|GetNearbyPickupActors _asglobal_map_character))
          (:Is%20Valid
            (Rendering|SetVisibility (Variables|BP_PickUpActor_C|GetPickUpText (Utilities|Array|Get(acopy) (Variables|/Game/Characters/GlobalMapCharacter/GlobalMapCharacter.GlobalMapCharacter_C|GetNearbyPickupActors _asglobal_map_character))) true false)))
        (else
          (Utilities|Array|RemoveItem (Variables|/Game/Characters/GlobalMapCharacter/GlobalMapCharacter.GlobalMapCharacter_C|GetNearbyPickupActors _asglobal_map_character) self))))
    (:then_1
      (bind _aslocal_map_character (Utilities|Casting|CastToLocalMapCharacter OtherActor))
      (Variables|Default|SetIsInRange? false)
      (if (and (Utilities|IsValid (Utilities|Array|Get(acopy) (Variables|/Game/Characters/LocalMapCharacter/LocalMapCharacter.LocalMapCharacter_C|GetNearbyPickupActors _aslocal_map_character))) (== (Utilities|Array|Get(acopy) (Variables|/Game/Characters/LocalMapCharacter/LocalMapCharacter.LocalMapCharacter_C|GetNearbyPickupActors _aslocal_map_character)) self))
        (Rendering|SetVisibility (Variables|Default|GetPickUpText) false false)
        (Utilities|Array|RemoveItem (Variables|/Game/Characters/LocalMapCharacter/LocalMapCharacter.LocalMapCharacter_C|GetNearbyPickupActors _aslocal_map_character) self)
        (Utilities|IsValid (Utilities|Array|Get(acopy) (Variables|/Game/Characters/LocalMapCharacter/LocalMapCharacter.LocalMapCharacter_C|GetNearbyPickupActors _aslocal_map_character))
          (:Is%20Valid
            (Rendering|SetVisibility (Variables|BP_PickUpActor_C|GetPickUpText (Utilities|Array|Get(acopy) (Variables|/Game/Characters/LocalMapCharacter/LocalMapCharacter.LocalMapCharacter_C|GetNearbyPickupActors _aslocal_map_character))) true false)))
        (else
          (Utilities|Array|RemoveItem (Variables|/Game/Characters/LocalMapCharacter/LocalMapCharacter.LocalMapCharacter_C|GetNearbyPickupActors _aslocal_map_character) self))))))

(event OnComponentBeginOverlap(Sphere)
  (params (OverlappedComponent :type Primitive%20Component%20Object%20Reference) (OtherActor :type Actor%20Object%20Reference) (OtherComp :type Primitive%20Component%20Object%20Reference) (OtherBodyIndex :type Integer) (bFromSweep :type Boolean) (SweepResult :type Hit%20Result%20Structure%20%28by%20ref%29))
  (Utilities|FlowControl|Sequence
    (:then_0
      (bind _asglobal_map_character (Utilities|Casting|CastToGlobalMapCharacter OtherActor))
      (if (Variables|Default|GetHasPickUpCommand?)
        (CallFunction|OnPickUp _asglobal_map_character)
        (elif (> (Utilities|Array|Length (Variables|/Game/Characters/GlobalMapCharacter/GlobalMapCharacter.GlobalMapCharacter_C|GetNearbyPickupActors _asglobal_map_character)) 0)
          (Utilities|Array|Add (Variables|/Game/Characters/GlobalMapCharacter/GlobalMapCharacter.GlobalMapCharacter_C|GetNearbyPickupActors _asglobal_map_character) self)
          (else
            (Rendering|SetVisibility (Variables|Default|GetPickUpText) true false)
            (Utilities|Array|Add (Variables|/Game/Characters/GlobalMapCharacter/GlobalMapCharacter.GlobalMapCharacter_C|GetNearbyPickupActors _asglobal_map_character) self)
            (Variables|Default|SetIsInRange? true)))))
    (:then_1
      (bind _aslocal_map_character (Utilities|Casting|CastToLocalMapCharacter OtherActor))
      (if (Variables|Default|GetHasPickUpCommand?)
        (CallFunction|OnPickUp 0 _aslocal_map_character)
        (elif (> (Utilities|Array|Length (Variables|/Game/Characters/LocalMapCharacter/LocalMapCharacter.LocalMapCharacter_C|GetNearbyPickupActors _aslocal_map_character)) 0)
          (Utilities|Array|Add (Variables|/Game/Characters/LocalMapCharacter/LocalMapCharacter.LocalMapCharacter_C|GetNearbyPickupActors _aslocal_map_character) self)
          (else
            (Rendering|SetVisibility (Variables|Default|GetPickUpText) true false)
            (Utilities|Array|Add (Variables|/Game/Characters/LocalMapCharacter/LocalMapCharacter.LocalMapCharacter_C|GetNearbyPickupActors _aslocal_map_character) self)
            (Variables|Default|SetIsInRange? true)))))))

(event OnEndCursorOver(StatickMesh)
  (params (TouchedComponent :type Primitive%20Component%20Object%20Reference))
  (Utilities|IsValid (Variables|Default|GetGlobalMapCharacter)
    (:Is%20Valid
      (CallFunction|OnUnHovered))))

(event Custom|OnPickUp
  (params (GlobalMapCharacter :type Global%20Map%20Character%20Object%20Reference) (LocalMapCharacter :type Local%20Map%20Character%20Object%20Reference))
  (bind _inventoryref (Variables|/Game/Characters/GlobalMapCharacter/GlobalMapCharacter.GlobalMapCharacter_C|GetInventoryRef GlobalMapCharacter))
  (bind _nearbypickupactors (Variables|/Game/Characters/GlobalMapCharacter/GlobalMapCharacter.GlobalMapCharacter_C|GetNearbyPickupActors GlobalMapCharacter))
  (bind _inventoryref_2 (Variables|/Game/Characters/GlobalMapCharacter/GlobalMapCharacter.GlobalMapCharacter_C|GetInventoryRef GlobalMapCharacter))
  (bind _output (Utilities|Array|Get(acopy) _nearbypickupactors))
  (Utilities|IsValid GlobalMapCharacter
    (:Is%20Valid
      (Utilities|IsValid _inventoryref
        (:Is%20Valid
          (bind (_succes _rest1) (Default|AddItem _inventoryref (Variables|Default|GetItemToAdd) (Variables|Default|GetAmount) true))
          (if _succes
            (if (> _rest1 0)
              (Variables|Default|SetAmount _rest1)
              (CallFunction|UpdateText)
              (Utilities|Array|Add (Variables|/Game/InventorySystem/Blueprints/BP_Inventory.BP_Inventory_C|GetLootedPickUps _inventoryref_2) (Utilities|Struct|MakeS_SavedPickUp (Variables|Default|GetID) (Variables|Default|GetAmount)))
              (else
                (Utilities|Array|Add (Variables|/Game/InventorySystem/Blueprints/BP_Inventory.BP_Inventory_C|GetLootedPickUps _inventoryref_2) (Utilities|Struct|MakeS_SavedPickUp (Variables|Default|GetID) 0))
                (Utilities|Array|RemoveItem _nearbypickupactors self)
                (Utilities|IsValid _output
                  (:Is%20Valid
                    (Rendering|SetVisibility (Variables|BP_PickUpActor_C|GetPickUpText _output) true false))
                  (:Is%20Not%20Valid
                    _))
                (if (Variables|Default|GetHovered?)
                  (Variables|/Script/Engine.PlayerController|SetCurrentMouseCursor (Game|GetPlayerController 0) "Default")
                  (Actor|DestroyActor)
                  (else
                    (Actor|DestroyActor)))))))))
    (:Is%20Not%20Valid
      (Variables|Default|SetLocalMapCharacter LocalMapCharacter)
      (Utilities|IsValid (Variables|/Game/Characters/LocalMapCharacter/LocalMapCharacter.LocalMapCharacter_C|GetInventoryRef (Variables|Default|GetLocalMapCharacter))
        (:Is%20Valid
          (bind (_succes_2 _rest1_2) (Default|AddItem (Variables|/Game/Characters/LocalMapCharacter/LocalMapCharacter.LocalMapCharacter_C|GetInventoryRef (Variables|Default|GetLocalMapCharacter)) (Variables|Default|GetItemToAdd) (Variables|Default|GetAmount) true))
          (if _succes_2
            (if (> _rest1_2 0)
              (Variables|Default|SetAmount _rest1_2)
              (CallFunction|UpdateText)
              (Utilities|Array|Add (Variables|/Game/InventorySystem/Blueprints/BP_Inventory.BP_Inventory_C|GetLootedPickUps (Variables|/Game/Characters/LocalMapCharacter/LocalMapCharacter.LocalMapCharacter_C|GetInventoryRef (Variables|Default|GetLocalMapCharacter))) (Utilities|Struct|MakeS_SavedPickUp (Variables|Default|GetID) (Variables|Default|GetAmount)))
              (else
                (Utilities|Array|Add (Variables|/Game/InventorySystem/Blueprints/BP_Inventory.BP_Inventory_C|GetLootedPickUps (Variables|/Game/Characters/LocalMapCharacter/LocalMapCharacter.LocalMapCharacter_C|GetInventoryRef (Variables|Default|GetLocalMapCharacter))) (Utilities|Struct|MakeS_SavedPickUp (Variables|Default|GetID) 0))
                (Utilities|Array|RemoveItem (Variables|/Game/Characters/LocalMapCharacter/LocalMapCharacter.LocalMapCharacter_C|GetNearbyPickupActors (Variables|Default|GetLocalMapCharacter)) self)
                (Utilities|IsValid (Utilities|Array|Get(acopy) (Variables|/Game/Characters/LocalMapCharacter/LocalMapCharacter.LocalMapCharacter_C|GetNearbyPickupActors (Variables|Default|GetLocalMapCharacter)))
                  (:Is%20Valid
                    (Rendering|SetVisibility (Variables|BP_PickUpActor_C|GetPickUpText (Utilities|Array|Get(acopy) (Variables|/Game/Characters/LocalMapCharacter/LocalMapCharacter.LocalMapCharacter_C|GetNearbyPickupActors (Variables|Default|GetLocalMapCharacter)))) true false))
                  (:Is%20Not%20Valid
                    _))
                (Actor|DestroyActor)))))))))

(event EventBeginPlay
  (bind _outactors (Actor|GetAllActorsOfClass "/Game/Characters/GlobalMapCharacter/GlobalMapCharacter.GlobalMapCharacter_C"))
  (Variables|Default|SetGlobalMapCharacter (Utilities|Array|Get(acopy) _outactors))
  (Utilities|IsValid (Variables|Default|GetGlobalMapCharacter)
    (:Is%20Valid
      (Variables|/Script/Engine.PlayerController|SetbEnableMouseOverEvents (Game|GetPlayerController 0) true)
      (CallFunction|UpdateText))
    (:Is%20Not%20Valid
      (CallFunction|UpdateText))))

(event Collision|EventActorBeginOverlap
  (params (OtherActor :type Actor%20Object%20Reference)))

(event EventTick
  (params (DeltaSeconds :type Float%20%28single-precision%29)))

(fn ConstructionScript
  (bind _itemtoadd (Variables|Default|GetItemToAdd))
  (bind _statickmesh (Variables|Default|GetStatickMesh))
  (bind _iteminfo (Utilities|GetClassDefaults _itemtoadd))
  (bind (_name _descriprion _icon _canbeused_ _usedtext _canbestacked_ _category _weight _recipe _value _pickupmesh _meshscale _interactradius) (Utilities|Struct|BreakS_ItemInfo _iteminfo))
  (if (Utilities|IsValidClass _itemtoadd)
    (Components|StaticMesh|SetStaticMesh _statickmesh _pickupmesh)
    (Variables|Default|SetOriginalMeterial (Rendering|Material|GetMaterial _statickmesh 0))
    (Transformation|SetRelativeScale3D _statickmesh _meshscale)
    (Components|Sphere|SetSphereRadius (Variables|Default|GetSphere) _interactradius false)))

(fn UpdateText
  (bind _aspick_up_text (Utilities|Casting|CastToPickUpText (UserInterface|GetUserWidgetObject (Variables|Default|GetPickUpText)))
    (:then
      (Rendering|Components|TextRender|SetText (Variables|/Game/InventorySystem/Widgets/PickUpText.PickUpText_C|GetNameText _aspick_up_text) (Utilities|Text|FormatText "{Name}({Amount})" (.Name (Utilities|Struct|BreakS_ItemInfo (.ItemInfo (Utilities|GetClassDefaults (Variables|Default|GetItemToAdd))))) (Utilities|Text|ToText(Integer) (Variables|Default|GetAmount)))))
    (:CastFailed
      _))
  (return))

(fn OnHovered
  (Variables|Default|SetHovered? true)
  (Variables|/Script/Engine.PlayerController|SetCurrentMouseCursor (Game|GetPlayerController 0) "Hand")
  (Rendering|Material|SetMaterial (Variables|Default|GetStatickMesh) 0 "/Game/InventorySystem/Materials/HoveredPickUpMat.HoveredPickUpMat")
  (Rendering|SetVisibility (Variables|Default|GetPickUpText) true false)
  (return))

(fn OnUnHovered
  (Variables|Default|SetHovered? false)
  (Variables|/Script/Engine.PlayerController|SetCurrentMouseCursor (Game|GetPlayerController 0) "Default")
  (Rendering|Material|SetMaterial (Variables|Default|GetStatickMesh) 0 (Variables|Default|GetOriginalMeterial))
  (Rendering|SetVisibility (Variables|Default|GetPickUpText) (Variables|Default|GetIsInRange?) false)
  (return))