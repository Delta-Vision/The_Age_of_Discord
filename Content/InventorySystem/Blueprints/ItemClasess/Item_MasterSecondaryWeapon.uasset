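; Base item class for secondary weapons in the inventory system, handling what happens when the item is used.
; On use, it asks the inventory's global-map character to equip it in the secondary slot, falling back to the local-map character when that one is not valid.
; If the equip call returns false, the item actor destroys itself.
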(event EventBeginPlay)

(event Collision|EventActorBeginOverlap
  (params (OtherActor :type Actor%20Object%20Reference)))

(event EventTick
  (params (DeltaSeconds :type Float%20%28single-precision%29)))

(event EventEventonUsed
  (Utilities|IsValid (Variables|/Game/InventorySystem/Blueprints/BP_Inventory.BP_Inventory_C|GetGlobalMapCharacter (Variables|Default|GetInventory))
    (:Is%20Valid
      (bind _succes_ (Default|EquipSecondaryItem (Variables|/Game/InventorySystem/Blueprints/BP_Inventory.BP_Inventory_C|GetGlobalMapCharacter (Variables|Default|GetInventory)) self false))
      (if (not _succes_)
        (Actor|DestroyActor)))
    (:Is%20Not%20Valid
      (bind _succes__2 (Default|EquipSecondaryItem (Variables|/Game/InventorySystem/Blueprints/BP_Inventory.BP_Inventory_C|GetLocalMapCharacter (Variables|Default|GetInventory)) self false))
      (if (not _succes__2)
        (Actor|DestroyActor)))))

(fn ConstructionScript
  (|CallParentFunction))