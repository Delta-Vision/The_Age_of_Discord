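; Interactable chest that opens a storage inventory for global-map or local-map characters.
; On BeginPlay it can roll starting loot from a data table using per-row chance and amount range.
; Overlapping the interaction range shows a prompt and registers the chest as nearby.
; Interacting lazily spawns a reusable BP_Storage, shows it alongside the inventory and disables movement, with a DoOnce blocking re-entry until closing restores movement.
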(event OnComponentBeginOverlap(InteractionRange)
  (params (OverlappedComponent :type Primitive%20Component%20Object%20Reference) (OtherActor :type Actor%20Object%20Reference) (OtherComp :type Primitive%20Component%20Object%20Reference) (OtherBodyIndex :type Integer) (bFromSweep :type Boolean) (SweepResult :type Hit%20Result%20Structure%20%28by%20ref%29))
  (Utilities|FlowControl|Sequence
    (:then_0
      (bind _asglobal_map_character (Utilities|Casting|CastToGlobalMapCharacter OtherActor))
      (Rendering|SetVisibility (Variables|Default|GetChestText) true false)
      (Variables|/Game/Characters/GlobalMapCharacter/GlobalMapCharacter.GlobalMapCharacter_C|SetNearbyChest _asglobal_map_character self))
    (:then_1
      (bind _aslocal_map_character (Utilities|Casting|CastToLocalMapCharacter OtherActor))
      (Rendering|SetVisibility (Variables|Default|GetChestText) true false)
      (Variables|/Game/Characters/LocalMapCharacter/LocalMapCharacter.LocalMapCharacter_C|SetNearbyChest _aslocal_map_character self))))

(event OnComponentEndOverlap(InteractionRange)
  (params (OverlappedComponent :type Primitive%20Component%20Object%20Reference) (OtherActor :type Actor%20Object%20Reference) (OtherComp :type Primitive%20Component%20Object%20Reference) (OtherBodyIndex :type Integer))
  (Utilities|FlowControl|Sequence
    (:then_0
      (bind _asglobal_map_character (Utilities|Casting|CastToGlobalMapCharacter OtherActor))
      (Rendering|SetVisibility (Variables|Default|GetChestText) false false)
      (Variables|/Game/Characters/GlobalMapCharacter/GlobalMapCharacter.GlobalMapCharacter_C|SetNearbyChest _asglobal_map_character 0))
    (:then_1
      (bind _aslocal_map_character (Utilities|Casting|CastToLocalMapCharacter OtherActor))
      (Rendering|SetVisibility (Variables|Default|GetChestText) false false)
      (Variables|/Game/Characters/LocalMapCharacter/LocalMapCharacter.LocalMapCharacter_C|SetNearbyChest _aslocal_map_character 0))))

(event Custom|OnStorageClosed
  (Utilities|IsValid (Variables|Default|GetGlobalMapCharacter)
    (:Is%20Valid
      (Default|HideStorage (Variables|Default|GetStorageRef))
      (Pawn|Components|CharacterMovement|SetMovementMode (Variables|/Script/Engine.Character|GetCharacterMovement (Variables|Default|GetGlobalMapCharacter)) "MOVE_Walking" 0)
      (if (Variables|/Game/InventorySystem/Blueprints/BP_Inventory.BP_Inventory_C|GetIsVisible? (Variables|/Game/Characters/GlobalMapCharacter/GlobalMapCharacter.GlobalMapCharacter_C|GetInventoryRef (Variables|Default|GetGlobalMapCharacter)))
        (Default|HideInventory (Variables|/Game/Characters/GlobalMapCharacter/GlobalMapCharacter.GlobalMapCharacter_C|GetInventoryRef (Variables|Default|GetGlobalMapCharacter)))
        (Default|ShowInventory (Variables|/Game/Characters/GlobalMapCharacter/GlobalMapCharacter.GlobalMapCharacter_C|GetInventoryRef (Variables|Default|GetGlobalMapCharacter)))
        (Utilities|FlowControl|DoOnce false) ; enters at Reset
        (else
          (Utilities|FlowControl|DoOnce false) ; enters at Reset
        )))
    (:Is%20Not%20Valid
      (Default|HideStorage (Variables|Default|GetStorageRef))
      (Pawn|Components|CharacterMovement|SetMovementMode (Variables|/Script/Engine.Character|GetCharacterMovement (Variables|Default|GetLocalMapCharacter)) "MOVE_Walking" 0)
      (if (Variables|/Game/InventorySystem/Blueprints/BP_Inventory.BP_Inventory_C|GetIsVisible? (Variables|/Game/Characters/LocalMapCharacter/LocalMapCharacter.LocalMapCharacter_C|GetInventoryRef (Variables|Default|GetLocalMapCharacter)))
        (Default|HideInventory (Variables|/Game/Characters/LocalMapCharacter/LocalMapCharacter.LocalMapCharacter_C|GetInventoryRef (Variables|Default|GetLocalMapCharacter)))
        (Default|ShowInventory (Variables|/Game/Characters/LocalMapCharacter/LocalMapCharacter.LocalMapCharacter_C|GetInventoryRef (Variables|Default|GetLocalMapCharacter)))
        (Utilities|FlowControl|DoOnce false) ; enters at Reset
        (else
          (Utilities|FlowControl|DoOnce false) ; enters at Reset
        )))))

(event Custom|OnInteract
  (params (GlobalMapCharacterChraracter :type Global%20Map%20Character%20Object%20Reference) (LocalMapCharacter :type Local%20Map%20Character%20Object%20Reference))
  (Utilities|FlowControl|DoOnce false
    (:Completed
      (Utilities|IsValid GlobalMapCharacterChraracter
        (:Is%20Valid
          (Variables|Default|SetGlobalMapCharacter GlobalMapCharacterChraracter)
          (Utilities|IsValid (Variables|Default|GetStorageRef)
            (:Is%20Valid
              _)
            (:Is%20Not%20Valid
              (bind _returnvalue (Game|SpawnActorfromClass "/Game/InventorySystem/Blueprints/BP_Storage.BP_Storage_C" (Math|Transform|MakeTransform "0, 0, 0" "0, 0, 0" "1,1,1") "AlwaysSpawn" 0 (Variables|Default|GetAmountOfSlots) (Variables|Default|GetGlobalMapCharacter) (Variables|Default|GetSlotsPerRow) self (Variables|Default|GetStartingItems) 0 0))
              (Variables|Default|SetStorageRef _returnvalue)))
          (Default|GenerateSlotWhidgets (Variables|/Game/InventorySystem/Blueprints/BP_Storage.BP_Storage_C|GetStorageWidget (Variables|Default|GetStorageRef)) (Variables|Default|GetStorageRef))
          (Default|ShowStorage (Variables|Default|GetStorageRef))
          (Default|HideInventory (Variables|/Game/Characters/GlobalMapCharacter/GlobalMapCharacter.GlobalMapCharacter_C|GetInventoryRef (Variables|Default|GetGlobalMapCharacter)))
          (Default|ShowInventory (Variables|/Game/Characters/GlobalMapCharacter/GlobalMapCharacter.GlobalMapCharacter_C|GetInventoryRef (Variables|Default|GetGlobalMapCharacter)))
          (Pawn|Components|CharacterMovement|DisableMovement (Variables|/Script/Engine.Character|GetCharacterMovement (Variables|Default|GetGlobalMapCharacter)))
          (Components|Movement|StopMovementImmediately (Variables|/Script/Engine.Character|GetCharacterMovement (Variables|Default|GetGlobalMapCharacter))))
        (:Is%20Not%20Valid
          (Variables|Default|SetLocalMapCharacter LocalMapCharacter)
          (Utilities|IsValid (Variables|Default|GetStorageRef)
            (:Is%20Valid
              _)
            (:Is%20Not%20Valid
              (bind _returnvalue_2 (Game|SpawnActorfromClass "/Game/InventorySystem/Blueprints/BP_Storage.BP_Storage_C" (Math|Transform|MakeTransform "0, 0, 0" "0, 0, 0" "1,1,1") "AlwaysSpawn" 0 (Variables|Default|GetAmountOfSlots) 0 (Variables|Default|GetSlotsPerRow) self (Variables|Default|GetStartingItems) (Variables|Default|GetLocalMapCharacter) 0))
              (Variables|Default|SetStorageRef _returnvalue_2)))
          (Default|GenerateSlotWhidgets (Variables|/Game/InventorySystem/Blueprints/BP_Storage.BP_Storage_C|GetStorageWidget (Variables|Default|GetStorageRef)) (Variables|Default|GetStorageRef))
          (Default|ShowStorage (Variables|Default|GetStorageRef))
          (Default|HideInventory (Variables|/Game/Characters/LocalMapCharacter/LocalMapCharacter.LocalMapCharacter_C|GetInventoryRef (Variables|Default|GetLocalMapCharacter)))
          (Default|ShowInventory (Variables|/Game/Characters/LocalMapCharacter/LocalMapCharacter.LocalMapCharacter_C|GetInventoryRef (Variables|Default|GetLocalMapCharacter)))
          (Pawn|Components|CharacterMovement|DisableMovement (Variables|/Script/Engine.Character|GetCharacterMovement (Variables|Default|GetLocalMapCharacter)))
          (Components|Movement|StopMovementImmediately (Variables|/Script/Engine.Character|GetCharacterMovement (Variables|Default|GetLocalMapCharacter))))))))

(event Collision|EventActorBeginOverlap
  (params (OtherActor :type Actor%20Object%20Reference)))

(event EventTick
  (params (DeltaSeconds :type Float%20%28single-precision%29)))

(event EventBeginPlay
  (if (Variables|Default|GetGenerateStrtingItmes?)
    (CallFunction|GenerateStartingItems)))

(fn ConstructionScript)

(fn GenerateStartingItems
  (bind _outrownames (DataTable|GetDataTableRowNames "/Game/InventorySystem/Blueprints/DataTables/Table_ChestStartItems.Table_ChestStartItems"))
  (for _array_element _outrownames
    (bind _returnvalue (Utilities|GetDataTableRow "/Game/InventorySystem/Blueprints/DataTables/Table_ChestStartItems.Table_ChestStartItems" _array_element)
      (:then
        (if (and (<= (Math|Random|RandomIntegerinRange 1 100) (.Chance (Utilities|Struct|BreakS_ChestContent _returnvalue))) (Utilities|IsValidClass (.ItemClass (Utilities|Struct|BreakS_ChestContent _returnvalue))))
          (Utilities|Array|Add (Variables|Default|GetStartingItems) (Utilities|Struct|MakeS_InventorySlot (.ItemClass (Utilities|Struct|BreakS_ChestContent _returnvalue)) (Math|Random|RandomIntegerinRange (.MinAmount (Utilities|Struct|BreakS_ChestContent _returnvalue)) (.MaxAmount (Utilities|Struct|BreakS_ChestContent _returnvalue)))))))))
  (return))